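; Player character Blueprint for a shooting game, handling the HUD, shot effects and the lose condition.
; BeginPlay creates the Mira and MyLife widgets, and Tick shows the Youlose widget and pauses the game when Vidas equals zero.
; Start and end shoot events toggle the Firing flag and a particle system, while the Shoot component's OnHit spawns a small explosion at the hit point.
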(event OnHit(shoot)
  (params (HitPoint :type Vector :default "0, 0, 0"))
  (Effects|SpawnEmitteratLocation "/Game/StarterContent/Particles/P_Explosion.P_Explosion" HitPoint "0, 0, 0" "0.100000,0.100000,0.100000"))

(event EventTick
  (params (DeltaSeconds :type Float%20%28single-precision%29))
  (if (== (Variables|Default|Getvidas) 0.0)
    (bind _returnvalue (UserInterface|CreateWidget "/Game/Contenido/Interfaz/Youlose.Youlose_C"))
    (UserInterface|Viewport|AddtoPlayerScreen _returnvalue)
    (Game|SetGamePaused true)))

(event EventOnStartShoot
  (Variables|Default|SetFiring true)
  (Components|Activation|Activate (Variables|Default|GetParticleSystem) false))

(event EventOnEndShoot
  (Variables|Default|SetFiring false)
  (Components|Activation|Deactivate (Variables|Default|GetParticleSystem)))

(event EventBeginPlay
  (CallFunction|CrearHUD)
  (bind _returnvalue (UserInterface|CreateWidget "/Game/Contenido/Interfaz/MyLife.MyLife_C"))
  (UserInterface|Viewport|AddtoPlayerScreen _returnvalue))

(fn ConstructionScript)

(fn CrearHUD
  (bind _returnvalue (UserInterface|CreateWidget "/Game/Contenido/Interfaz/Mira.Mira_C"))
  (UserInterface|Viewport|AddtoViewport _returnvalue 0))